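; Spikes hazard actor that kills the ChibiBP character when it overlaps the Box trigger.
; The construction script sets the UpDawn interp movement between relative Up and Dawn control points, with Time as its duration.
; On overlap it calls PlayerDied on the character, then after a short delay destroys that character and removes all widgets.
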(event `self.Box.OnComponentBeginOverlap`
  (params (OverlappedComponent :type "PrimitiveComponent Object Reference") (OtherActor :type "Actor Object Reference") (OtherComp :type "PrimitiveComponent Object Reference") (OtherBodyIndex :type Integer) (bFromSweep :type Boolean) (SweepResult :type "HitResult Structure (by ref)"))
  (bind _aschibi_bp (cast `/Game/Chibi/ChibiBP` OtherActor))
  (`/Game/Chibi/ChibiBP.PlayerDied` _aschibi_bp)
  (`KismetSystemLibrary.Delay` 3.5)
  (`self.K2_DestroyActor` _aschibi_bp)
  (`WidgetLayoutLibrary.RemoveAllWidgets`))

(fn `UserConstructionScript`
  (bind _updawn (`self.UpDawn`))
  (set `InterpToMovementComponent.ControlPoints` (`|MakeArray` (make `InterpControlPoint` (`self.Up`)) (make `InterpControlPoint` (`self.Dawn`))) _updawn)
  (set `InterpToMovementComponent.Duration` (`self.Time`) _updawn))