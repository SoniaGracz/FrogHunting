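; Coins is a collectible coin Blueprint that flies toward the ChibiBP character that touches it.
; An overlap on the Erte component starts a timeline, which lerps the Coin component from its current position toward the character's live location, producing a homing pull.
; When the timeline finishes, it calls CollectedCoin on the character, plays the coin sound at the coin and destroys the actor.
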(event `self.erte.OnComponentBeginOverlap`
  (params (OverlappedComponent :type "PrimitiveComponent Object Reference") (OtherActor :type "Actor Object Reference") (OtherComp :type "PrimitiveComponent Object Reference") (OtherBodyIndex :type Integer) (bFromSweep :type Boolean) (SweepResult :type "HitResult Structure (by ref)"))
  (bind _returnvalue (`SceneComponent.K2_GetComponentLocation` (`self.Coin`)))
  (bind _aschibi_bp (cast `/Game/Chibi/ChibiBP` OtherActor))
  (set `self.LocationCoin` _returnvalue)
  (bind (_direction _newtrack_0) (`Timeline|Timeline_0`)
    (:`Update`
      (bind _returnvalue_2 (`KismetMathLibrary.VLerp` _returnvalue (`self.K2_GetActorLocation` _aschibi_bp) _newtrack_0))
      (`SceneComponent.K2_SetWorldLocation` (`self.Coin`) _returnvalue_2 false false))
    (:`Finished`
      (`/Game/Chibi/ChibiBP.CollectedCoin` _aschibi_bp)
      (`GameplayStatics.PlaySoundAtLocation` "/Game/Sounds/CoinSound.CoinSound" _returnvalue_2 (struct) 1.0 1.0 0.0 null null null)
      (`self.K2_DestroyActor`))))

(fn `UserConstructionScript`)