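; A checkpoint actor that saves the player's respawn location in the game mode.
; When ChibiBP overlaps the box, it copies that character's transform into ThirdPersonGameMode's SpawnTransform and sets a Respawn flag.
; The first touch also swaps CubeDirtSingle's materials to CheckpointAfter and restarts the Click interp movement, which is halted at BeginPlay.
; The construction script builds that movement's relative control points and duration from Up, Dawn and Time variables.
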(event `self.ReceiveBeginPlay`
  (`MovementComponent.StopMovementImmediately` (`self.Click`)))

(event `self.Box.OnComponentBeginOverlap`
  (params (OverlappedComponent :type "PrimitiveComponent Object Reference") (OtherActor :type "Actor Object Reference") (OtherComp :type "PrimitiveComponent Object Reference") (OtherBodyIndex :type Integer) (bFromSweep :type Boolean) (SweepResult :type "HitResult Structure (by ref)"))
  (bind _aschibi_bp (cast `/Game/Chibi/ChibiBP` OtherActor))
  (bind _asthird_person_game_mode (cast `/Game/Blueprints/ThirdPersonGameMode` (`GameplayStatics.GetGameMode`)))
  (set `/Game/Blueprints/ThirdPersonGameMode.SpawnTransform` (`self.GetTransform` _aschibi_bp) _asthird_person_game_mode)
  (set `self.Respawn?` true)
  (if (not (`self.Clicked`))
    (for _index (range 3)
      (`PrimitiveComponent.SetMaterial` (`self.Cube_Dirt_Single`) _index "/Game/Materials/CheckpointAfter.CheckpointAfter")
      (`InterpToMovementComponent.RestartMovement` (`self.Click`) 1.0)
      (set `self.Clicked` true))))

(fn `UserConstructionScript`
  (bind _click (`self.Click`))
  (set `InterpToMovementComponent.ControlPoints` (`|MakeArray` (make `InterpControlPoint` (`self.Up`)) (make `InterpControlPoint` (`self.Dawn`))) _click)
  (set `InterpToMovementComponent.Duration` (`self.Time`) _click))