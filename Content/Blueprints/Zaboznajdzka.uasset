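; Frog collectible that moves between two configurable relative points through an interp movement component set up in the construction script.
; When the ChibiBP character overlaps it, it calls CollectedFrog on that character, spawns a particle burst, plays a frog sound and destroys itself.
; A short delay meant to remove the particle component follows the DestroyActor call.
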(event `self.r.OnComponentBeginOverlap`
  (params (OverlappedComponent :type "PrimitiveComponent Object Reference") (OtherActor :type "Actor Object Reference") (OtherComp :type "PrimitiveComponent Object Reference") (OtherBodyIndex :type Integer) (bFromSweep :type Boolean) (SweepResult :type "HitResult Structure (by ref)"))
  (bind _returnvalue (`self.K2_GetActorLocation`))
  (bind _aschibi_bp (cast `/Game/Chibi/ChibiBP` OtherActor))
  (bind _returnvalue_2 (`GameplayStatics.SpawnEmitterAtLocation` "/Game/Particles/Zaba.Zaba" _returnvalue))
  (set `self.ParticleSystem` _returnvalue_2)
  (`/Game/Chibi/ChibiBP.Collected Frog` _aschibi_bp)
  (`self.K2_DestroyActor`)
  (`GameplayStatics.PlaySoundAtLocation` "/Game/Sounds/FrogSound.FrogSound" _returnvalue (struct) 1.0 1.0 0.0 null null null)
  (`KismetSystemLibrary.Delay` 0.2)
  (`ActorComponent.K2_DestroyComponent` (`self.ParticleSystem`)))

(fn `UserConstructionScript`
  (bind _updawn (`self.UpDawn`))
  (set `InterpToMovementComponent.ControlPoints` (`|MakeArray` (make `InterpControlPoint` (`self.Up`)) (make `InterpControlPoint` (`self.Dawn`))) _updawn)
  (set `InterpToMovementComponent.Duration` (`self.Time`) _updawn))