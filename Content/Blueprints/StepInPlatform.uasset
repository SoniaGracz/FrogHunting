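; Moving platform that stays still until the ChibiBP character steps into its overlap volume.
; The construction script builds two relative control points from Forward and Backward and sets the movement duration from Time.
; The first overlap restarts the interpolated movement.
; Tick resets and halts it whenever the player's X is at or below a hard-coded threshold, using a restart, short delay and stop.
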(event `self.ReceiveBeginPlay`
  (`MovementComponent.StopMovementImmediately` (`self.Move`)))

(event `self.rer.OnComponentBeginOverlap`
  (params (OverlappedComponent :type "PrimitiveComponent Object Reference") (OtherActor :type "Actor Object Reference") (OtherComp :type "PrimitiveComponent Object Reference") (OtherBodyIndex :type Integer) (bFromSweep :type Boolean) (SweepResult :type "HitResult Structure (by ref)"))
  (cast `/Game/Chibi/ChibiBP` OtherActor)
  (if (not (`self.Moving?`))
    (`InterpToMovementComponent.RestartMovement` (`self.Move`) 1.0)
    (set `self.Moving?` true)))

(event `self.ReceiveTick`
  (params (DeltaSeconds :type "Float (single-precision)"))
  (bind _aschibi_bp (cast `/Game/Chibi/ChibiBP` (`GameplayStatics.GetPlayerCharacter` 0)))
  (if (not (> (.x (`self.K2_GetActorLocation` _aschibi_bp)) -3300.0))
    (`MovementComponent.StopMovementImmediately` (`self.Move`))
    (`InterpToMovementComponent.RestartMovement` (`self.Move`) 1.0)
    (`KismetSystemLibrary.Delay` 0.1)
    (`MovementComponent.StopMovementImmediately` (`self.Move`))
    (set `self.Moving?` false)))

(fn `UserConstructionScript`
  (bind _move (`self.Move`))
  (set `InterpToMovementComponent.ControlPoints` (`|MakeArray` (make `InterpControlPoint` (`self.Forward`)) (make `InterpControlPoint` (`self.Backward`))) _move)
  (set `InterpToMovementComponent.Duration` (`self.Time`) _move))